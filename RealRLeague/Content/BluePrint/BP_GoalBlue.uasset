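; BP_GoalBlue is the blue team's goal, which detects when the ball enters it and awards the point to the red team.
; An overlap on GoalDetector checks for the Ball class, prints a goal message and calls the ball's ResetPositions.
; It then casts the first player's HUD to NewHUDDD to call CalcScore for TeamRed and plays applause, printing an error if that cast fails.
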(event `self.ReceiveActorBeginOverlap`
  (params (OtherActor :type "Actor Object Reference")))

(event `self.GoalDetector.OnComponentBeginOverlap`
  (params (OtherActor :type "Actor Object Reference") (OtherComp :type "PrimitiveComponent Object Reference") (OtherBodyIndex :type Integer) (bFromSweep :type Boolean) (SweepResult :type "HitResult Structure (by ref)"))
  (if (== "/Game/BluePrint/Ball.Ball_C" (`GameplayStatics.GetObjectClass` OtherActor))
    (`KismetSystemLibrary.PrintString` "GOAL!")
    (bind _asball (cast `/Game/BluePrint/Ball` OtherActor))
    (`/Game/BluePrint/Ball.Reset Positions` _asball)
    ;[1 0.5048 0.8897] Makes use of the function CalcScore, from NewHUDDD
    (bind _asnew_huddd (cast `/Game/Widget/NewHUDDD` (`PlayerController.GetHUD` (`GameplayStatics.GetPlayerController` 0)))
      (:`then`
        (`/Game/Widget/NewHUDDD.CalcScore` _asnew_huddd (`self.TeamRed`))
        (`GameplayStatics.PlaySound2D` "/Game/Sound/Applause.Applause" 0.6))
      (:`CastFailed`
        (`KismetSystemLibrary.PrintString` "Fail to cast to NewHUDDD") ; If it can't cast to the function CalcScore, it prints this string to the screen
      ))))

(fn `UserConstructionScript`)